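; BP_Mechanika is an actor that swings back and forth in a fixed vertical plane, like a pendulum.
; Tick accumulates time into a sine wave set by Chastota (frequency) and Amplitude, driving the Y offset around a hard-coded centre.
; Z derives from the square of that offset, so the path is a parabola that rises toward both ends.
; SetActorLocation applies absolute coordinates without sweep, with X held constant.
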(event `self.ReceiveBeginPlay`)

(event `self.ReceiveActorBeginOverlap`
  (params (OtherActor :type "Actor Object Reference")))

(event `self.ReceiveTick`
  (params (DeltaSeconds :type "Float (single-precision)"))
  (bind _output_get (set `self.Timer` (+ DeltaSeconds (`self.Timer`))))
  (bind _returnvalue (* (`KismetMathLibrary.Sin` (* (`KismetMathLibrary.MultiplyByPi` (/ _output_get (/ 1.0 (`self.chastota`)))) 2.0)) (`self.amplitude`)))
  (`self.K2_SetActorLocation` (`KismetMathLibrary.MakeVector` 410.0 (+ _returnvalue -210.0) (- (- 575.0 (/ (- 1.0 (* _returnvalue _returnvalue)) 575.0)) 400.0))))

(fn `UserConstructionScript`)