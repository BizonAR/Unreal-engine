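; BP_Mechanika is an actor that bobs up and down in a continuous sine-wave oscillation.
; Tick accumulates a timer and feeds it into a sine, with Chastota as the frequency and Amplituda as the amplitude.
; The result offsets Z around a hardcoded world position, applied through a swept SetActorLocation, so the actor's placed location is ignored during play.
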(event `self.ReceiveBeginPlay`)

(event `self.ReceiveActorBeginOverlap`
  (params (OtherActor :type "Actor Object Reference")))

(event `self.ReceiveTick`
  (params (DeltaSeconds :type "Float (single-precision)"))
  (bind _output_get (set `self.Timer` (+ DeltaSeconds (`self.Timer`))))
  (`self.K2_SetActorLocation` (`KismetMathLibrary.MakeVector` 290.0 -40.0 (+ (* (`KismetMathLibrary.Sin` (* (`KismetMathLibrary.MultiplyByPi` (/ _output_get (/ 1.0 (`self.chastota`)))) 2.0)) (`self.amplituda`)) 300.0)) true))

(fn `UserConstructionScript`)