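; BP_Mechanika is an actor that moves along a horizontal circle at constant frequency, apparently a uniform circular motion demo.
; Each Tick accumulates Timer and converts it to an angle of 2π × time × Chastota (frequency).
; Sine and cosine of that angle, scaled by radius XCenter − X, offset the actor from XCenter and YCenter at fixed height ZCenter via SetActorLocation without sweep.
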(event `/Game/BP_physicsUE_1.ReceiveBeginPlay`)

(event `self.ReceiveActorBeginOverlap`
  (params (OtherActor :type "Actor Object Reference")))

(event `self.ReceiveTick`
  (params (DeltaSeconds :type "Float (single-precision)"))
  (bind _returnvalue (- (`self.X_center`) (`self.x`)))
  (bind _output_get (set `self.Timer` (+ DeltaSeconds (`self.Timer`))))
  (bind _returnvalue_2 (* (`KismetMathLibrary.MultiplyByPi` (/ _output_get (/ 1.0 (`self.chastota`)))) 2.0))
  (`self.K2_SetActorLocation` (`KismetMathLibrary.MakeVector` (+ (* (`KismetMathLibrary.Sin` _returnvalue_2) _returnvalue) (`self.X_center`)) (+ (* _returnvalue (`KismetMathLibrary.Cos` _returnvalue_2)) (`self.Y_center`)) (`self.Z_center`))))

(fn `UserConstructionScript`)